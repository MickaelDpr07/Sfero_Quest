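; BP_ky_fireBall is a fireball projectile actor that spawns a color-tinted shockwave effect when it begins play.
; Tick moves it along local X, with speed scaled by a timeline curve, and counts down its lifetime.
; A delay loop watches that countdown, then disables collision, deactivates the effect and destroys the actor a second later.
; Overlapping an actor whose first tag isn't "ky_shot" spawns a hit effect and destroys it immediately.
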(event `self.ReceiveBeginPlay`
  (bind _defaultsceneroot (`self.DefaultSceneRoot`))
  ;[0.2422 0 1] spawn shot shockwave
  (bind _returnvalue (`GameplayStatics.SpawnEmitterAtLocation` "/Game/FXVarietyPack/Particles/P_ky_shotShockwave.P_ky_shotShockwave" (`SceneComponent.K2_GetComponentLocation` _defaultsceneroot) (`SceneComponent.K2_GetComponentRotation` _defaultsceneroot)))
  (`ParticleSystemComponent.SetVectorParameter` _returnvalue "color" (`KismetMathLibrary.Conv_LinearColorToVector` (`self.color`)))
  ;[1 0.6797 0] effect move correct
  (bind (_direction _valuecorrect) (`Timeline|Timeline_0`)
    (:`Update`
      (set `self.speedCorrect` _valuecorrect)
      ;[0 0.5312 1] duration control
      (`KismetSystemLibrary.Delay` 0.1 :!label _label)
      (if (< (`self.duration`) 0.0)
        ;[0.6641 1 0] fx deactivate
        (`PrimitiveComponent.SetCollisionEnabled` (`self.Box`) "NoCollision")
        (`ActorComponent.Deactivate` (`self.FX1`))
        (`KismetSystemLibrary.Delay` 1.0)
        ;[0.8281 0 1] effect destroy
        (`self.K2_DestroyActor`)
        (else
          (goto _label))))))

(event `self.ReceiveTick`
  (params (DeltaSeconds :type "Float (single-precision)"))
  ;[0 1 0.25] duration increment for control
  (set `self.duration` (- (`self.duration`) DeltaSeconds))
  ;[0.3359 1 0] move control
  (`self.K2_AddActorLocalOffset` (`KismetMathLibrary.MakeVector` (* (`self.speed`) (`self.speedCorrect`) (`GameplayStatics.GetWorldDeltaSeconds`)))))

(event `self.ReceiveActorBeginOverlap`
  (params (OtherActor :type "Actor Object Reference"))
  ;[0 0.7891 1] spawn collison fx
  (if (`KismetSystemLibrary.IsValid` OtherActor)
    (if (!= (`|GetArrayItem` (`Actor.Tags` OtherActor)) "ky_shot")
      (`GameplayStatics.SpawnEmitterAtLocation` (`self.hitFx`) (`SceneComponent.K2_GetComponentLocation` (`self.Box`)))
      ;[1 0 0.1875] fx destroy
      (`self.K2_DestroyActor`))))

(fn `UserConstructionScript`)