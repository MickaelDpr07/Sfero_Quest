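; One-shot trigger actor that launches a tutorial step screen when the player's sphere (BP_Sféro) enters its collision volume.
; BeginPlay caches the player pawn and the GM_Sféro game mode.
; On overlap it removes the game mode's main widget, shows WB_EtapeTuto with the texture picked from ListeEtapes by IndexEtape, then destroys itself.
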(event `self.ReceiveBeginPlay`
  ;[0.5469 1 0] Références
  (bind `_asbp_sféro` (cast `/Game/SpheroQuest/Core/BP_Sféro` (`GameplayStatics.GetPlayerPawn` 0)))
  (set `self.BP Sféro` `_asbp_sféro`)
  (bind `_asgm_sféro` (cast `/Game/SpheroQuest/Core/GM_Sféro` (`GameplayStatics.GetGameMode`)))
  (set `self.GM Sféro` `_asgm_sféro`))

(event `self.Collision_Overlap.OnComponentBeginOverlap`
  (params (OverlappedComponent :type "PrimitiveComponent Object Reference") (OtherActor :type "Actor Object Reference") (OtherComp :type "PrimitiveComponent Object Reference") (OtherBodyIndex :type Integer) (bFromSweep :type Boolean) (SweepResult :type "HitResult Structure (by ref)"))
  (if (== OtherActor (`self.BP Sféro`))
    (`Widget.RemoveFromParent` (`/Game/SpheroQuest/Core/GM_Sféro.WB_Main` (`self.GM Sféro`)))
    (bind _returnvalue (`|CreateWidget` "/Game/SpheroQuest/Widgets/WB_EtapeTuto.WB_EtapeTuto_C"))
    (`UserWidget.AddToViewport` _returnvalue 0)
    (`Image.SetBrushFromTexture` (`/Game/SpheroQuest/Widgets/WB_EtapeTuto.IMG_TUTO` _returnvalue) (`|GetArrayItem` (`self.Liste_Etapes`) (`self.IndexEtape`)) false)
    (`self.K2_DestroyActor`)))

(fn `UserConstructionScript`)