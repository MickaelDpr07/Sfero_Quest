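; Parent Blueprint for elemental surfaces whose TypeDamage sets the cube's material in the Construction Script and gates its reaction to effects.
; MagmaEffect on a Magma-type surface with a valid cube attaches a firestorm actor, then destroys the surface after a short delay.
; On other types it attaches a "can't effect" actor and prints a message.
; Only the Magma reaction is implemented; the CantEffetSphère function is empty.
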(event `/Game/SpheroQuest/Core/Scientist/BPI_Damageable.MagmaEffect`
  ;[1 0.3588 0] MAGMA
  (if (`|EnumEquality` (`self.TypeDamage`) "NewEnumerator0")
    (`/Engine/EditorBlueprintResources/StandardMacros.IsValid` (`self.SurfaceCube`)
      (:`Is Valid`
        (bind _returnvalue (`|SpawnActorFromClass` "/Game/FXVarietyPack/Blueprints/BP_ky_fireStorm.BP_ky_fireStorm_C" (`KismetMathLibrary.MakeTransform` (0.0 0.0 -30.0) (struct) (1.0 0.5 0.25)) "Undefined" "MultiplyWithRoot" null null))
        (`self.K2_AttachToComponent` _returnvalue (`self.SurfaceCube`) "None" "KeepRelative" "KeepRelative" "KeepRelative" true)
        (`KismetSystemLibrary.Delay` 3.0)
        (`self.K2_DestroyActor`)))
    (else
      ;;[0.05469 0 1] NS Can't Effet sur Ennemi
      (bind _returnvalue_2 (`|SpawnActorFromClass` "/Game/FXVarietyPack/Blueprints/BP_ky_CantEffect.BP_ky_CantEffect_C" (`KismetMathLibrary.MakeTransform` (0.0 0.0 0.0) (struct) (0.5 0.5 0.5)) "Undefined" "MultiplyWithRoot" null null))
      (`self.K2_AttachToComponent` _returnvalue_2 (`self.SurfaceCube`) "None" "KeepRelative" "KeepRelative" "KeepRelative" true)
      (`KismetSystemLibrary.PrintString` "Can't Effet"))))

(fn `Can't Effet Sphère`)

(fn `UserConstructionScript`
  (`PrimitiveComponent.SetMaterial` (`self.SurfaceCube`) 0 (select `/Game/SpheroQuest/Core/ENUM_Inventaire` (`self.TypeDamage`) :`NewEnumerator0` "/Game/SpheroQuest/Core/SurfacesBP/MI_Magma.MI_Magma" :`NewEnumerator1` "/Game/SpheroQuest/Core/SurfacesBP/MI_Geltra.MI_Geltra" :`NewEnumerator2` "/Game/SpheroQuest/Core/SurfacesBP/MI_Briz.MI_Briz" :`NewEnumerator3` "/Game/SpheroQuest/Core/SurfacesBP/MI_Géolithe.MI_Géolithe" :!type "MaterialInterface Object Reference")))