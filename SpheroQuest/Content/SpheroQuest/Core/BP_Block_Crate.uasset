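; BP_Block_Crate is a destructible crate block in SpheroQuest that wears down when hit by projectiles.
; Each TakeDamage call removes one HealthPoint; at zero or below, it spawns the NS_Explosion Niagara effect at its location and destroys the actor.
; Otherwise, reaching CrackThreshold swaps in the cracked crate texture through FUpdateTexture, guarded by a DoOnce so it happens only once.
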(event `/Game/SpheroQuest/Core/BPI_Damageable.TakeDamage`
  ;[1 1 1] Gère la prise de dégat lorsqu'on est touché par un projectile
  (bind _result (`/Engine/EditorBlueprintResources/StandardMacros.DecrementInt` (`self.HealthPoints`))
    (:`  `
      (if (<= _result 0)
        (`NiagaraFunctionLibrary.SpawnSystemAtLocation` "/Game/SpheroQuest/Core/NS_Explosion.NS_Explosion" (`self.K2_GetActorLocation`))
        (`self.K2_DestroyActor`)
        (elif (<= (`self.HealthPoints`) (`self.CrackThreshold`))
          (`/Engine/EditorBlueprintResources/StandardMacros.DoOnce` false
            (:`Completed`
              (`self.f_Update Texture` "/Game/SpheroQuest/Art/Interactables/Crate/T_Crate_Cracked.T_Crate_Cracked"))))))))

(fn `UserConstructionScript`
  (`parent.UserConstructionScript`))