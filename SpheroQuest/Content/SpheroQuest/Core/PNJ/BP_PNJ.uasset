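; BP_PNJ is a placeable NPC for SpheroQuest that tells the game mode when the player's sphere is in talking range.
; The construction script picks the Paper2D sprite and overhead name text from the NPC name enum.
; Tick polls the collision sphere for overlap with BP_Sféro, using enter/exit flags to update GM_Sféro's current interaction and NPC only on transitions, clearing the NPC on exit.
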(event `self.ReceiveBeginPlay`
  ;[1 0.375 0] Références
  (bind `_asgm_sféro` (cast `/Game/SpheroQuest/Core/GM_Sféro` (`GameplayStatics.GetGameMode`)))
  (set `self.GM Sféro` `_asgm_sféro`)
  (bind `_asbp_sféro` (cast `/Game/SpheroQuest/Core/BP_Sféro` (`GameplayStatics.GetPlayerPawn` 0)))
  (set `self.BP Sféro` `_asbp_sféro`))

(event `self.ReceiveTick`
  (params (DeltaSeconds :type "Float (single-precision)"))
  (if (`PrimitiveComponent.IsOverlappingActor` (`self.SphèreCollision`) (`self.BP Sféro`))
    (if (`self.Est Sortit`)
      (set `self.Est Sortit` false)
      (set `self.Est Entrer` true)
      (set `/Game/SpheroQuest/Core/GM_Sféro.InteractionActu` "NewEnumerator0" (`self.GM Sféro`))
      (set `/Game/SpheroQuest/Core/GM_Sféro.PNJ_Actu` (`self.Nom_PNJ`) (`self.GM Sféro`))
      (`KismetSystemLibrary.PrintString` "Set PNJ"))
    (elif (`self.Est Entrer`)
      (set `self.Est Entrer` false)
      (set `self.Est Sortit` true)
      (set `/Game/SpheroQuest/Core/GM_Sféro.InteractionActu` "NewEnumerator2" (`self.GM Sféro`))
      (set `/Game/SpheroQuest/Core/GM_Sféro.PNJ_Actu` "NewEnumerator4" (`self.GM Sféro`))
      (`KismetSystemLibrary.PrintString` "NONE PNJ"))))

(fn `UserConstructionScript`
  ;[1 0 0.1172] Set Sprite en fonction du PNJ à qui on parle
  (`PaperSpriteComponent.SetSprite` (`self.PaperSprite`) (select `/Game/SpheroQuest/Core/PNJ/ENUM_PNJ` (`self.Nom_PNJ`) :`NewEnumerator0` "/Game/SpheroQuest/Art/Habitants/Bergere_Sprite.Bergere_Sprite" :`NewEnumerator1` "/Game/SpheroQuest/Art/Habitants/Doyen_Sprite.Doyen_Sprite" :`NewEnumerator2` "/Game/SpheroQuest/Art/Habitants/Gentil_Scientifique_Sprite.Gentil_Scientifique_Sprite" :`NewEnumerator3` "/Game/SpheroQuest/Art/Habitants/Jardiniere_Sprite.Jardiniere_Sprite" :!type "PaperSprite Object Reference"))
  ;[0 1 0.03906] Set Nom au dessus en fonction du PNJ
  (`TextRenderComponent.K2_SetText` (`self.TXT_Nom`) (`KismetTextLibrary.Conv_StringToText` (`|GetEnumeratorNameAsString` (`self.Nom_PNJ`)))))