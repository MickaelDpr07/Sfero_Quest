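; BP_PowerBlocks is a configurable grid of instanced blocks that can be blown up in a chain reaction.
; The construction script builds the X/Y/Z grid in an InstancedStaticMesh and sizes and centres a slightly padded Box around it.
; TriggerExplosion starts a looping timer that removes one instance at a time, spawning a Niagara explosion and sound, until none remain and the timer is cleared.
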(event `TriggerExplosion`
  ;[1 1 1] Lance l'explosion en châine de tous les blocks de l'instance et les détruits
  (`self.DestroyOneInstance`)
  (bind _returnvalue (`KismetSystemLibrary.K2_SetTimerDelegate` (delegate `DestroyOneInstance`) 0.1 true))
  (set `self.Explosion Timer` _returnvalue))

(event `DestroyOneInstance`
  ;[1 1 1] Lance l'explosion en châine de tous les blocks de l'instance et les détruits
  (if (> (`InstancedStaticMeshComponent.GetInstanceCount` (`self.InstancedStaticMesh`)) 0)
    (`NiagaraFunctionLibrary.SpawnSystemAtLocation` "/Game/SpheroQuest/Core/NS_Explosion.NS_Explosion" (.location (`InstancedStaticMeshComponent.GetInstanceTransform` (`self.InstancedStaticMesh`) 0 true)))
    (`InstancedStaticMeshComponent.RemoveInstance` (`self.InstancedStaticMesh`) 0)
    (`GameplayStatics.SpawnSound2D` "/Game/SpheroQuest/Audio/A_Explode.A_Explode" 0.5 0.8 0.0 null)
    (else
      (`KismetSystemLibrary.K2_ClearAndInvalidateTimerHandle` (`self.Explosion Timer`)))))

(fn `UserConstructionScript`
  (bind _box (`self.Box`))
  (bind _returnvalue (`KismetMathLibrary.MakeVector` (`KismetMathLibrary.Conv_IntToDouble` (`self.NumX`)) (`KismetMathLibrary.Conv_IntToDouble` (`self.NumY`)) (`KismetMathLibrary.Conv_IntToDouble` (`self.NumZ`))))
  (`|ExecutionSequence`
    (:`then_0`
      ;[1 1 1] Crée des blocks de manières procédurale
      (`InstancedStaticMeshComponent.ClearInstances` (`self.InstancedStaticMesh`))
      (for _index (range (`self.NumZ`))
        (for _index_2 (range (`self.NumY`))
          (for _index_3 (range (`self.NumX`))
            (`InstancedStaticMeshComponent.AddInstance` (`self.InstancedStaticMesh`) (`KismetMathLibrary.MakeTransform` (`KismetMathLibrary.MakeVector` (* _index_3 100.0) (* _index_2 100.0) (* _index 100.0))) false)))))
    (:`then_1`
      (`BoxComponent.SetBoxExtent` _box (+ (* _returnvalue 50.0) 10.0) true)
      (`SceneComponent.K2_SetRelativeLocation` _box (* (- _returnvalue 1.0) 50.0) false false))))