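; BP_Loot_Sphère is a pickup actor that lets the player's Sféro loot a sphere.
; On BeginPlay it caches the player pawn as BP_Sféro and the game mode as GM_Sféro.
; When that pawn overlaps Sphere_Loot, it passes SphereÀLoot to InitilisationImages on the sphere inventory widget held by the game mode's main widget.
; The graph only updates that widget and never destroys the actor.
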(event `self.ReceiveBeginPlay`
  ;[0 0.8125 1] Références
  (bind `_asbp_sféro` (cast `/Game/SpheroQuest/Core/BP_Sféro` (`GameplayStatics.GetPlayerPawn` 0)))
  (set `self.BP Sféro` `_asbp_sféro`)
  (bind `_asgm_sféro` (cast `/Game/SpheroQuest/Core/GM_Sféro` (`GameplayStatics.GetGameMode`)))
  (set `self.GM Sféro` `_asgm_sféro`))

(event `self.Sphere_Loot.OnComponentBeginOverlap`
  (params (OverlappedComponent :type "PrimitiveComponent Object Reference") (OtherActor :type "Actor Object Reference") (OtherComp :type "PrimitiveComponent Object Reference") (OtherBodyIndex :type Integer) (bFromSweep :type Boolean) (SweepResult :type "HitResult Structure (by ref)"))
  (if (== OtherActor (`self.BP Sféro`))
    (`/Game/SpheroQuest/Widgets/WB_Inventaire_Spheres.Initilisation Images` (`/Game/SpheroQuest/Widgets/WB_MAIN.WB_Inventaire_Spheres` (`/Game/SpheroQuest/Core/GM_Sféro.WB_Main` (`self.GM Sféro`))) (`self.Sphere à loot`))))

(fn `UserConstructionScript`)