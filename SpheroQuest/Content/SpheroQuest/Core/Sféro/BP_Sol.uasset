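; BP_Sol is a procedural ground Blueprint that builds a solid grid of blocks sized by NumX, NumY and NumZ.
; The construction script clears and refills an InstancedStaticMesh with one instance per cell, spaced 100 units apart.
; It then sizes and centers a Box component around the grid, with a 10-unit margin beyond the nominal block bounds.
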(fn `UserConstructionScript`
  (bind _box (`self.Box`))
  (bind _returnvalue (`KismetMathLibrary.MakeVector` (`KismetMathLibrary.Conv_IntToDouble` (`self.NumX`)) (`KismetMathLibrary.Conv_IntToDouble` (`self.NumY`)) (`KismetMathLibrary.Conv_IntToDouble` (`self.NumZ`))))
  (`|ExecutionSequence`
    (:`then_0`
      ;[1 0.6797 0] Crée des blocks de manières procédurale
      (`InstancedStaticMeshComponent.ClearInstances` (`self.InstancedStaticMesh`))
      (for _index (range (`self.NumZ`))
        (for _index_2 (range (`self.NumY`))
          (for _index_3 (range (`self.NumX`))
            (`InstancedStaticMeshComponent.AddInstance` (`self.InstancedStaticMesh`) (`KismetMathLibrary.MakeTransform` (`KismetMathLibrary.MakeVector` (* _index_3 100.0) (* _index_2 100.0) (* _index 100.0))) false)))))
    (:`then_1`
      (`BoxComponent.SetBoxExtent` _box (+ (* _returnvalue 50.0) 10.0) true)
      (`SceneComponent.K2_SetRelativeLocation` _box (* (- _returnvalue 1.0) 50.0) false false))))