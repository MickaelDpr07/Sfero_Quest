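; Player character for SpheroQuest that draws a trailing chain of instanced spheres as it moves.
; Enhanced Input drives movement along the forward vector and jumping with a 2D sound.
; The construction script lays out NBSphères instances on a detached instanced mesh component.
; While velocity exceeds a small threshold, Tick snaps the first sphere to the actor and lerps each following one toward its predecessor's snapshotted transform, creating a snake-like lag.
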(event `self.ReceiveBeginPlay`
  ;[0 1 0.0625] Définit la config des touches par défault du jeu
  (`EnhancedInputSubsystemInterface.AddMappingContext` (pcsubsystem `EnhancedInputLocalPlayerSubsystem` (`GameplayStatics.GetPlayerController` 0)) "/Game/SpheroQuest/Core/Inputs/IMC_Default.IMC_Default" 0 (struct)))

(event `EnhancedInput|/Game/SpheroQuest/Core/Inputs/INP_MoveAround`
  (params (ActionValue :type "Float (double-precision)") (ElapsedSeconds :type "Float (double-precision)") (TriggeredSeconds :type "Float (double-precision)") (InputAction :type "InputAction Object Reference" :default "/Game/SpheroQuest/Core/Inputs/INP_MoveAround.INP_MoveAround"))
  ;[1 0 0.4687] Gère les déplacements
  (:`Triggered`
    (`self.AddMovementInput` (`self.GetActorForwardVector`) ActionValue)))

(event `EnhancedInput|/Game/SpheroQuest/Core/Inputs/INP_Jump`
  (params (ActionValue :type Boolean) (ElapsedSeconds :type "Float (double-precision)") (TriggeredSeconds :type "Float (double-precision)") (InputAction :type "InputAction Object Reference" :default "/Game/SpheroQuest/Core/Inputs/INP_Jump.INP_Jump"))
  (bind _charactermovement (`self.CharacterMovement`))
  ;[0.5 0 1] Gère le saut
  (:`Started`
    (`self.Jump`)
    (if (`KismetMathLibrary.BooleanNOR` (`NavMovementComponent.IsFalling` _charactermovement) (`NavMovementComponent.IsCrouching` _charactermovement))
      (`GameplayStatics.SpawnSound2D` "/Game/SpheroQuest/Audio/A_Jump.A_Jump" 0.3 1.0 0.0 null)))
  (:`Completed`
    (`self.StopJumping`)))

(event `self.ReceiveTick`
  (params (DeltaSeconds :type "Float (single-precision)"))
  ;[1 0 0 1 30] EVENT TICK
  (if (> (`KismetMathLibrary.VSize` (`self.GetVelocity`)) 10.0)
    (`self.LerpLocations`)))

(event `LerpLocations`
  (bind (_returnvalue_location _returnvalue_rotation) (`KismetMathLibrary.BreakTransform` (`self.GetTransform`)))
  (bind (_output_location _output_rotation _output_scale) (`KismetMathLibrary.BreakTransform` (`|GetArrayItem` (`self.Instance_Transforms`))))
  (`KismetArrayLibrary.Array_Clear` (`self.Instance_Transforms`))
  (for _index (range (`InstancedStaticMeshComponent.GetInstanceCount` (`self.ISM_Sphères`)))
    (`KismetArrayLibrary.Array_Add` (`self.Instance_Transforms`) (`InstancedStaticMeshComponent.GetInstanceTransform` (`self.ISM_Sphères`) _index true)))
  (`InstancedStaticMeshComponent.UpdateInstanceTransform` (`self.ISM_Sphères`) 0 (`KismetMathLibrary.MakeTransform` _returnvalue_location _returnvalue_rotation _output_scale) true true false)
  (for (_array_element _array_index) (`self.Instance_Transforms`)
    (bind _returnvalue (+ _array_index 1))
    (`InstancedStaticMeshComponent.UpdateInstanceTransform` (`self.ISM_Sphères`) _returnvalue (`KismetMathLibrary.TLerp` (`InstancedStaticMeshComponent.GetInstanceTransform` (`self.ISM_Sphères`) _returnvalue true) _array_element 0.05) true false false)))

(fn `UserConstructionScript`
  (`SceneComponent.K2_DetachFromComponent` (`self.ISM_Sphères`) "KeepWorld" "KeepWorld" "KeepWorld" true)
  (`InstancedStaticMeshComponent.ClearInstances` (`self.ISM_Sphères`))
  (for _index (range 1 (+ (`self.NB_Sphères`) 1))
    (`InstancedStaticMeshComponent.AddInstance` (`self.ISM_Sphères`) (`KismetMathLibrary.MakeTransform` (`KismetMathLibrary.MakeVector` (`KismetMathLibrary.Conv_IntToDouble` (* _index -75))) (struct) (0.75 0.75 0.75)) false)))