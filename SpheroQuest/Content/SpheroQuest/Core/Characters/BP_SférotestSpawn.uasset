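; Test player character for SpheroQuest that spawns a trailing chain of physics-linked spheres on BeginPlay.
; Each spawned BP_Sphères is offset along world X and stored in an array.
; Its PhysicsConstraint ties the first sphere to the Sféro component and each later one to the previous sphere.
; Enhanced Input drives forward-axis movement and jumping, with a jump sound unless falling or crouching.
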(event `self.ReceiveBeginPlay`
  (`|ExecutionSequence`
    (:`then_0`
      ;[0 1 0.0625] Définit la config des touches par défault du jeu
      (`EnhancedInputSubsystemInterface.AddMappingContext` (pcsubsystem `EnhancedInputLocalPlayerSubsystem` (`GameplayStatics.GetPlayerController` 0)) "/Game/SpheroQuest/Core/Inputs/IMC_Default.IMC_Default" 0 (struct)))
    (:`then_1`
      (for _index (range 1 (+ (`self.NB_Sphères`) 1))
        (`self.Spawn_Actor_Set_Position_Constraint` _index)))))

(event `EnhancedInput|/Game/SpheroQuest/Core/Inputs/INP_MoveAround`
  (params (ActionValue :type "Float (double-precision)") (ElapsedSeconds :type "Float (double-precision)") (TriggeredSeconds :type "Float (double-precision)") (InputAction :type "InputAction Object Reference" :default "/Game/SpheroQuest/Core/Inputs/INP_MoveAround.INP_MoveAround"))
  ;[1 0 0.4687] Gère les déplacements
  (:`Triggered`
    (`self.AddMovementInput` (`self.GetActorForwardVector`) ActionValue)))

(event `EnhancedInput|/Game/SpheroQuest/Core/Inputs/INP_Jump`
  (params (ActionValue :type Boolean) (ElapsedSeconds :type "Float (double-precision)") (TriggeredSeconds :type "Float (double-precision)") (InputAction :type "InputAction Object Reference" :default "/Game/SpheroQuest/Core/Inputs/INP_Jump.INP_Jump"))
  (bind _charactermovement (`self.CharacterMovement`))
  ;[0.5 0 1] Gère le saut
  (:`Started`
    (`self.Jump`)
    (if (`KismetMathLibrary.BooleanNOR` (`NavMovementComponent.IsFalling` _charactermovement) (`NavMovementComponent.IsCrouching` _charactermovement))
      (`GameplayStatics.SpawnSound2D` "/Game/SpheroQuest/Audio/A_Jump.A_Jump" 0.3 1.0 0.0 null)))
  (:`Completed`
    (`self.StopJumping`)))

(fn `Spawn_Actor_Set_Position_Constraint`
  (params (`IndexSphère` :type Integer))
  (bind _returnvalue (`self.GetTransform`))
  (bind _returnvalue_2 (* `IndexSphère` 80.0))
  (bind _returnvalue_3 (`|SpawnActorFromClass` "/Game/SpheroQuest/Core/Characters/BP_Sphères.BP_Sphères_C" (`KismetMathLibrary.MakeTransform` (`KismetMathLibrary.MakeVector` (- (.x (.location _returnvalue)) (select `int` `IndexSphère` :`0` 100.0 :`1` _returnvalue_2 :`2` _returnvalue_2 :`3` _returnvalue_2 :`4` _returnvalue_2 :!type "Float (single-precision)")) (.y (.location _returnvalue)) (.z (.location _returnvalue))) (.rotation _returnvalue)) "Undefined" "MultiplyWithRoot" null null))
  (bind _returnvalue_4 (`KismetArrayLibrary.Array_Add` (`self.SpawnsRéférences`) _returnvalue_3))
  (if (== _returnvalue_4 0)
    (bind _physicsconstraint (`/Game/SpheroQuest/Core/Characters/BP_Sphères.PhysicsConstraint` _returnvalue_3))
    (`SceneComponent.K2_SetRelativeLocation` _physicsconstraint (-20.0 0.0 0.0) false false)
    (bind _sphere (`/Game/SpheroQuest/Core/Characters/BP_Sphères.Sphere` _returnvalue_3))
    (`PhysicsConstraintComponent.SetConstrainedComponents` _physicsconstraint (`self.Sféro`) "None" _sphere "None")
    (else
      (`PhysicsConstraintComponent.SetConstrainedComponents` _physicsconstraint (`/Game/SpheroQuest/Core/Characters/BP_Sphères.Sphere` (`|GetArrayItem` (`self.SpawnsRéférences`) (- _returnvalue_4 1))) "None" _sphere "None"))))

(fn `UserConstructionScript`)