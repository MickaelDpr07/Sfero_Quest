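; Player character that moves along its forward axis, jumps with a sound and spawns a trailing BP_Sphères actor.
; BeginPlay adds the Enhanced Input context, then spawns the sphere 100 units behind on world X and stores it in SpawnsRéférences.
; Tick drives MoveComponentTo from an X-velocity test that passes for every value except exactly 10, so its stop branch rarely runs.
; A raised jump-follow event, MoveJumpSpawnActor, is defined but never called here.
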(event `self.ReceiveBeginPlay`
  (`|ExecutionSequence`
    (:`then_0`
      ;[0 1 0.0625] Définit la config des touches par défault du jeu
      (`EnhancedInputSubsystemInterface.AddMappingContext` (pcsubsystem `EnhancedInputLocalPlayerSubsystem` (`GameplayStatics.GetPlayerController` 0)) "/Game/SpheroQuest/Core/Inputs/IMC_Default.IMC_Default" 0 (struct)))
    (:`then_1`
      (`self.Spawn_Actor_Set_Position`))))

(event `EnhancedInput|/Game/SpheroQuest/Core/Inputs/INP_MoveAround`
  (params (ActionValue :type "Float (double-precision)") (ElapsedSeconds :type "Float (double-precision)") (TriggeredSeconds :type "Float (double-precision)") (InputAction :type "InputAction Object Reference" :default "/Game/SpheroQuest/Core/Inputs/INP_MoveAround.INP_MoveAround"))
  ;[1 0 0.4687] Gère les déplacements
  (:`Triggered`
    (`self.AddMovementInput` (`self.GetActorForwardVector`) ActionValue)))

(event `EnhancedInput|/Game/SpheroQuest/Core/Inputs/INP_Jump`
  (params (ActionValue :type Boolean) (ElapsedSeconds :type "Float (double-precision)") (TriggeredSeconds :type "Float (double-precision)") (InputAction :type "InputAction Object Reference" :default "/Game/SpheroQuest/Core/Inputs/INP_Jump.INP_Jump"))
  (bind _charactermovement (`self.CharacterMovement`))
  ;[0.5 0 1] Gère le saut
  (:`Started`
    (`self.Jump`)
    (if (`KismetMathLibrary.BooleanNOR` (`NavMovementComponent.IsFalling` _charactermovement) (`NavMovementComponent.IsCrouching` _charactermovement))
      (`GameplayStatics.SpawnSound2D` "/Game/SpheroQuest/Audio/A_Jump.A_Jump" 0.3 1.0 0.0 null)))
  (:`Completed`
    (`self.StopJumping`)))

(event `self.ReceiveTick`
  (params (DeltaSeconds :type "Float (single-precision)"))
  (bind _returnvalue_x (`KismetMathLibrary.BreakVector` (`self.K2_GetActorLocation`)))
  (bind _returnvalue_x_2 (`KismetMathLibrary.BreakVector` (`self.GetVelocity`)))
  (bind _output (`|GetArrayItem` (`self.SpawnsRéférences`)))
  (bind (_returnvalue_x_3 _returnvalue_y _returnvalue_z) (`KismetMathLibrary.BreakVector` (`self.K2_GetActorLocation` _output)))
  ;[1 0 0 1 30] EVENT TICK
  (if (or (> _returnvalue_x_2 10.0) (< _returnvalue_x_2 10.0))
    (`self.MoveSpawnActor`)
    (else
      (goto _label :!via `Stop`))))

(event `MoveSpawnActor`
  (bind _returnvalue_x (`KismetMathLibrary.BreakVector` (`self.K2_GetActorLocation`)))
  (bind _output (`|GetArrayItem` (`self.SpawnsRéférences`)))
  (bind (_returnvalue_x_2 _returnvalue_y _returnvalue_z) (`KismetMathLibrary.BreakVector` (`self.K2_GetActorLocation` _output)))
  (`KismetSystemLibrary.MoveComponentTo` (`Actor.RootComponent` _output) (`KismetMathLibrary.MakeVector` (- _returnvalue_x 100.0) _returnvalue_y _returnvalue_z) :!label _label))

(event `MoveJumpSpawnActor`
  (bind _returnvalue (`self.GetTransform`))
  (`KismetSystemLibrary.MoveComponentTo` (`Actor.RootComponent` (`|GetArrayItem` (`self.SpawnsRéférences`))) (`KismetMathLibrary.MakeVector` (- (.x (.location _returnvalue)) 100.0) 0.0 (+ (.z (.location _returnvalue)) 100.0))))

(fn `Spawn_Actor_Set_Position`
  (bind _returnvalue (`self.GetTransform`))
  (bind _returnvalue_2 (`|SpawnActorFromClass` "/Game/SpheroQuest/Core/Characters/BP_Sphères.BP_Sphères_C" (`KismetMathLibrary.MakeTransform` (`KismetMathLibrary.MakeVector` (- (.x (.location _returnvalue)) 100.0) (.y (.location _returnvalue)) (.z (.location _returnvalue))) (.rotation _returnvalue)) "Undefined" "MultiplyWithRoot" null null))
  (`KismetArrayLibrary.Array_Add` (`self.SpawnsRéférences`) _returnvalue_2))

(fn `UserConstructionScript`)